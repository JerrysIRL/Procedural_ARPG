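; Fireball projectile Blueprint that keeps its visual mesh turned toward the player's camera.
; On BeginPlay it starts a fast looping timer that calls FacePlayer, rather than using Tick.
; FacePlayer computes a look-at rotation from the actor to the first player's camera and adds a 90 degree pitch offset before applying it to the ProjectileMesh in world space, billboard style.
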(event `self.ReceiveBeginPlay`
  (`KismetSystemLibrary.K2_SetTimer` null "FacePlayer" 0.01 true))

(fn `FacePlayer`
  (`SceneComponent.K2_SetWorldRotation` (`self.ProjectileMesh`) (`KismetMathLibrary.MakeRotator` (.roll (`KismetMathLibrary.FindLookAtRotation` (`self.K2_GetActorLocation`) (`PlayerCameraManager.GetCameraLocation` (`GameplayStatics.GetPlayerCameraManager` 0)))) (+ (.pitch (`KismetMathLibrary.FindLookAtRotation` (`self.K2_GetActorLocation`) (`PlayerCameraManager.GetCameraLocation` (`GameplayStatics.GetPlayerCameraManager` 0)))) 90.0) (.yaw (`KismetMathLibrary.FindLookAtRotation` (`self.K2_GetActorLocation`) (`PlayerCameraManager.GetCameraLocation` (`GameplayStatics.GetPlayerCameraManager` 0))))) false false))

(fn `UserConstructionScript`)