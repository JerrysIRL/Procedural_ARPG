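; Ocean tile for grid-based world generation by cell collapse, overriding its selection weight based on neighbors and position.
; If any collapsed neighbor is ocean, ApplyUniqueWeightChanges scales the weight by center distance normalized to the half-diagonal, minus a high threshold and clamped.
; This sharply suppresses ocean beside ocean, leaving it near-zero everywhere except toward the grid corners.
; Without an ocean neighbor it returns -1.
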(fn `ApplyUniqueWeightChanges`
  (params (OwnerCell :type "Cell Object Reference") (Weight :type "Float (single-precision)") (GridSize :type Integer))
  (returns (ReturnValue :type "Float (single-precision)"))
  (locals (CenterOfWorld :type "Vector2D Structure"))
  (bind _returnvalue (`KismetMathLibrary.Conv_IntToDouble` (/ GridSize 2)))
  (for _array_element (`Cell.Neighbors` OwnerCell)
    (if (`Cell.bIsCollapsed` _array_element)
      (if (`KismetMathLibrary.ClassIsChildOf` (`.TileClass` (break `TileVariant` (`Cell.GetCollapsedTile` _array_element))) "BP_OceanTile_C")
        (bind _output_get (set `local.CenterOfWorld` (`KismetMathLibrary.MakeVector2D` _returnvalue _returnvalue)))
        (return (* Weight (`KismetMathLibrary.FClamp` (- (/ (`KismetMathLibrary.Abs` (`KismetMathLibrary.Distance2D` (`Cell.GridPosition` OwnerCell) _output_get)) (`KismetMathLibrary.Hypotenuse` _returnvalue _returnvalue)) 0.95) 0.0001))))))
  (return -1.0))

(fn `UserConstructionScript`)