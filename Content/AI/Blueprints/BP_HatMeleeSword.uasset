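; BP_HatMeleeSword is an AI character Blueprint, by its name a sword-wielding melee variant, that defines what happens when the character dies.
; HandleDeath stops the AI logic, plays a non-looping death animation directly on the mesh, then destroys the actor after a short delay.
; The other events are disabled default stubs, and the construction script only calls its parent.
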(event `self.HandleDeath`
  (params (Enemy :type "BaseEnemy Object Reference"))
  (`self.StopLogic`)
  (`SkeletalMeshComponent.PlayAnimation` (`self.Mesh`) "/Game/CityofBrass_Enemies/Meshes/Enemy/Corpse/animation/Corpse_Alert_Death.Corpse_Alert_Death" false)
  (`KismetSystemLibrary.Delay` 3.0)
  (`self.K2_DestroyActor`))

(fn `UserConstructionScript`
  (`parent.UserConstructionScript`))