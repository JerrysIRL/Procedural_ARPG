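; BP_Exploder is a suicide-bomber AI character that explodes to deal fire damage to the top-down player character.
; Attack plays the BombAttack gameplay cue, applies a fire-tagged damage spec if a small sphere overlap finds BP_TopDownCharacter, then calls OnPlayerDead on itself.
; HandleDeath plays the same cue, ragdolls, deactivates its particle system and destroys the actor after a short delay.
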(event `self.ReceiveBeginPlay`)

(event `self.ReceiveActorBeginOverlap`
  (params (OtherActor :type "Actor Object Reference")))

(event `self.HandleDeath`
  (params (Enemy :type "BaseEnemy Object Reference"))
  (`GameplayCueFunctionLibrary.ExecuteGameplayCueOnActor` self (struct :`TagName` "GameplayCue.BombAttack") (`AbilitySystemBlueprintLibrary.MakeGameplayCueParameters` 0.0))
  (`self.Ragdoll`)
  (`ActorComponent.Deactivate` (`self.ParticleSystem`))
  (`KismetSystemLibrary.Delay` 2.0)
  (`self.K2_DestroyActor`))

(fn `Attack`
  (`GameplayCueFunctionLibrary.ExecuteGameplayCueOnActor` self (struct :`TagName` "GameplayCue.BombAttack") (`AbilitySystemBlueprintLibrary.MakeGameplayCueParameters` 0.0))
  (bind (_outactors _returnvalue) (`KismetSystemLibrary.SphereOverlapActors` (`self.K2_GetActorLocation`) 100.0 (`|MakeArray`) "/Game/TopDown/Blueprints/BP_TopDownCharacter.BP_TopDownCharacter_C"))
  (if _returnvalue
    (bind _returnvalue_2 (`self.GetDamageSpec` (`self.BaseDamage`) (struct :`GameplayTags` (struct :`(TagName` "Damage.Element.Fire")))))
    (`self.ApplyDamage` _returnvalue_2))
  (`self.OnPlayerDead` self)
  (return))

(fn `UserConstructionScript`)