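; BP_MeteorStrike is a meteor attack actor that falls onto its own location and hits player 0 on impact.
; On BeginPlay, a timeline lerps MovingComp from its starting position to the actor location without sweeping.
; Impact uses a distance check rather than collision, applying the SpecHandle gameplay effect to the player's ability system if within HitRadius.
; It then deactivates the magic circle, spawns a hit emitter and destroys itself.
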(event `self.ReceiveBeginPlay`
  (set `self.StartPos` (`SceneComponent.K2_GetComponentLocation` (`self.MovingComp`)))
  (bind (_direction _moving_goal) (`Timeline|Lerp` :!via `PlayFromStart`)
    (:`Update`
      (`SceneComponent.K2_SetWorldLocation` (`self.MovingComp`) (`KismetMathLibrary.VLerp` (`self.StartPos`) (`self.K2_GetActorLocation`) _moving_goal) false false))
    (:`Finished`
      (`self.OnMeteorHit`))))

(event `OnMeteorHit`
  (bind _returnvalue (`GameplayStatics.GetPlayerCharacter` 0))
  (if (<= (`self.GetDistanceTo` self _returnvalue) (`self.HitRadius`))
    (`AbilitySystemComponent.BP_ApplyGameplayEffectSpecToSelf` (`AbilitySystemBlueprintLibrary.GetAbilitySystemComponent` _returnvalue) (`self.SpecHandle`)))
  (`ActorComponent.Deactivate` (`self.P_ky_magicCircle2`))
  (`GameplayStatics.SpawnEmitterAtLocation` "/Game/FXVarietyPack/Particles/P_ky_ThunderBallHit.P_ky_ThunderBallHit" (`self.K2_GetActorLocation`))
  (`self.K2_DestroyActor`))

(fn `UserConstructionScript`)