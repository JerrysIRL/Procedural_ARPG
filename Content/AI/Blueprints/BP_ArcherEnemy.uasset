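; Archer enemy character that fires arrow projectiles and handles its own death.
; Attack builds a physical-element damage spec from BaseDamage and passes it to a BP_Arrow spawned at the ProjectileSpawnPos transform.
; On death it stops its logic, plays a backward death animation, then destroys itself after a short delay.
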(event `self.ReceiveBeginPlay`)

(event `self.ReceiveTick`
  (params (DeltaSeconds :type "Float (single-precision)")))

(event `self.HandleDeath`
  (params (Enemy :type "BaseEnemy Object Reference"))
  (`self.StopLogic`)
  (`SkeletalMeshComponent.PlayAnimation` (`self.Mesh`) "/Game/AI/Animations/Archer/Standing_Death_Backward_01.Standing_Death_Backward_01" false)
  (`KismetSystemLibrary.Delay` 3.0)
  (`self.K2_DestroyActor`))

(fn `Attack`
  (bind _returnvalue (`self.GetDamageSpec` (`self.BaseDamage`) (struct :`GameplayTags` (struct :`(TagName` "Damage.Element.Physical")))))
  (`|SpawnActorFromClass` "/Game/AI/Blueprints/BP_Arrow.BP_Arrow_C" (`SceneComponent.K2_GetComponentToWorld` (`self.ProjectileSpawnPos`)) "AlwaysSpawn" "MultiplyWithRoot" null _returnvalue null)
  (return))

(fn `UserConstructionScript`)